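; Baseball actor that launches itself with a fixed impulse on spawn and resolves the play when it lands on Ground-tagged actors.
; Look input rotates its SpringArm for an orbiting ball view.
; An unhit ball reports a foul to GI_GameInstance, while a fouled hit just despawns.
; A fair hit blends the view back to BP_FirstPersonCharacter and opens run selection, with short delays before each outcome.
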(event `self.ReceiveBeginPlay`
  (`PrimitiveComponent.AddImpulse` (`self.Sphere`) (0.0 -250000.0 125000.0) "None" false))

(event `EnhancedInput|/Game/FirstPerson/Input/Actions/IA_Look`
  (params (ActionValue :type "Vector2D Structure") (ElapsedSeconds :type "Float (double-precision)") (TriggeredSeconds :type "Float (double-precision)") (InputAction :type "InputAction Object Reference" :default "/Game/FirstPerson/Input/Actions/IA_Look.IA_Look"))
  (:`Triggered`
    (bind _result (`/Engine/EditorBlueprintResources/StandardMacros.NegateFloat` ActionValue_Y)
      (:`  `
        (`SceneComponent.K2_AddRelativeRotation` (`self.SpringArm`) (`KismetMathLibrary.MakeRotator` 0.0 _result ActionValue_X) false false)))))

(event `self.Sphere.OnComponentHit`
  (params (HitComponent :type "PrimitiveComponent Object Reference") (OtherActor :type "Actor Object Reference") (OtherComp :type "PrimitiveComponent Object Reference") (NormalImpulse :type "Vector Structure") (Hit :type "HitResult Structure (by ref)"))
  (if (`self.IsActive`)
    (if (`self.ActorHasTag` OtherActor "Ground")
      (if (`self.HasBeenHit`)
        (if (`self.Fouled`)
          (set `self.IsActive` false)
          (`KismetSystemLibrary.Delay` 2.0)
          (`self.K2_DestroyActor`)
          (else
            (`KismetSystemLibrary.Delay` 2.0)
            (bind _returnvalue (`GameplayStatics.GetActorOfClass` "/Game/FirstPerson/Blueprints/BP_FirstPersonCharacter.BP_FirstPersonCharacter_C"))
            (`PlayerController.SetViewTargetWithBlend` (`GameplayStatics.GetPlayerController` 0) _returnvalue 0.2 "VTBlend_Linear" 0.0 false)
            (set `self.HasBeenHit` false)
            (bind _asgi_game_instance (cast `/Game/GI_GameInstance` (`GameplayStatics.GetGameInstance`)))
            (`/Game/GI_GameInstance.OpenRunSelection` _asgi_game_instance)
            (set `self.IsActive` false)
            (`self.K2_DestroyActor`)))
        (else
          (set `self.IsActive` false)
          (`KismetSystemLibrary.Delay` 2.0)
          (`self.K2_DestroyActor`)
          (bind _asgi_game_instance_2 (cast `/Game/GI_GameInstance` (`GameplayStatics.GetGameInstance`)))
          (`/Game/GI_GameInstance.FoulBall` _asgi_game_instance_2))))))

(fn `UserConstructionScript`)