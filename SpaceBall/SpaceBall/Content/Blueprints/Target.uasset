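; Target actor that scores a point in the game instance when a Baseball overlaps its Box, then redirects the ball.
; With TargetToBounceTo set, a timeline lerps the physics-disabled ball toward that target, chaining bounces; otherwise physics launches it along the Cube's negated right vector.
; LastTargetInBounce links back so an incoming hit can interrupt the previous timeline.
; A DoOnce blocks repeat scoring until the bounce or launch resets it.
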(event `self.Box.OnComponentBeginOverlap`
  (params (OverlappedComponent :type "PrimitiveComponent Object Reference") (OtherActor :type "Actor Object Reference") (OtherComp :type "PrimitiveComponent Object Reference") (OtherBodyIndex :type Integer) (bFromSweep :type Boolean) (SweepResult :type "HitResult Structure (by ref)"))
  (bind _lasttargetinbounce (`self.LastTargetInBounce`))
  (bind _asbaseball (cast `/Game/Blueprints/Baseball` OtherActor))
  (`/Engine/EditorBlueprintResources/StandardMacros.IsValid` _lasttargetinbounce
    (:`Is Valid`
      (`self.StopLastTimeline` _lasttargetinbounce))
    (:`Is Not Valid`
      _))
  (bind _sphere (`/Game/Blueprints/Baseball.Sphere` _asbaseball))
  (`PrimitiveComponent.SetSimulatePhysics` _sphere false)
  (`/Engine/EditorBlueprintResources/StandardMacros.DoOnce` false :!label _label
    (:`Completed`
      (bind _asgi_game_instance (cast `/Game/GI_GameInstance` (`GameplayStatics.GetGameInstance`)))
      (`/Engine/EditorBlueprintResources/StandardMacros.IncrementInt` (`/Game/GI_GameInstance.Score` _asgi_game_instance)
        (:`  `
          (`/Engine/EditorBlueprintResources/StandardMacros.IsValid` (`self.TargetToBounceTo`)
            (:`Is Valid`
              (bind (_direction _newtrack_1) (`Timeline|Timeline` :!via `PlayFromStart` :!label _label_2)
                (:`Update`
                  (`SceneComponent.K2_SetWorldLocation` _sphere (`KismetMathLibrary.VLerp` (`SceneComponent.K2_GetComponentLocation` _sphere) (`self.K2_GetActorLocation` (`self.TargetToBounceTo`)) _newtrack_1) false false))
                (:`Finished`
                  (`self.CanScoreAgain`)
                  (`PrimitiveComponent.SetSimulatePhysics` _sphere true))))
            (:`Is Not Valid`
              (`PrimitiveComponent.SetSimulatePhysics` _sphere true)
              (`PrimitiveComponent.SetAllPhysicsLinearVelocity` _sphere (* (`KismetMathLibrary.NegateVector` (`SceneComponent.GetRightVector` (`self.Cube`))) (1000.0 1000.0 1000.0)) false)
              (`self.CanScoreAgain`))))))))

(event `CanScoreAgain`
  (goto _label :!via `Reset`))

(event `StopLastTimeline`
  (bind _lasttargetinbounce (`self.LastTargetInBounce`))
  (`/Engine/EditorBlueprintResources/StandardMacros.IsValid` _lasttargetinbounce
    (:`Is Valid`
      (`self.CanScoreAgain` _lasttargetinbounce)
      (goto _label_2 :!via `Stop`))))

(fn `UserConstructionScript`)